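; BP_GizmoAccess is an actor providing a mouse-driven translation gizmo, with M toggling move mode and the cursor.
; Left click traces under the cursor, identifies the hit X, Y or Z axis component, and stores hit distance and grab offset.
; Tick deprojects the cursor at that distance and nudges GizmoRoot by a scaled delta projected onto the dragged axis's forward vector.
; Releasing the button clears the dragged axis.
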(event EventBeginPlay
  (Input|EnableInput (Game|GetPlayerController 0))
  (Development|PrintString "Press M to switch to gizmoz mode"))

(event Collision|EventActorBeginOverlap
  (params (OtherActor :type Actor%20Object%20Reference)))

(event EventTick
  (params (DeltaSeconds :type Float%20%28single-precision%29))
  (bind _returnvalue (Game|GetPlayerController 0))
  (bind (_worldlocation _worlddirection) (Game|Player|ConvertMouseLocationToWorldSpace _returnvalue))
  (Transformation|AddRelativeLocation (Variables|Default|GetGizmoRoot) (* (Math|Vector|ProjectVectorontoVector (Math|Transform|InverseTransformLocation (Math|Conversions|ToTransform(Vector) (Variables|Default|GetDragedLocation)) (+ _worldlocation (* _worlddirection (Variables|Default|GetDistanceToGraph)))) (Math|Vector|GetForwardVector (Variables|Default|GetAxis%20Draged))) 0.1) false false))

(event Input|MouseEvents|LeftMouseButton
  (params (Key :type Key%20Structure :default "None"))
  (bind _returnvalue (Game|GetPlayerController 0))
  (bind _movefunction (Variables|Default|GetMoveFunction))
  (bind (_worldlocation _worlddirection) (Game|Player|ConvertMouseLocationToWorldSpace _returnvalue))
  (:Pressed
    (if _movefunction
      (bind _outhit (Collision|LineTraceByChannel _worldlocation (+ _worldlocation (* _worlddirection 1e+04)) "TraceTypeQuery1" true 0 "ForDuration" false))
      (Variables|Default|SetDistanceToGraph (.Distance (Collision|BreakHitResult _outhit)))
      (switch Utilities|FlowControl|Switch|SwitchonAxisVariable (.axisvariable (Utilities|Struct|MakeDragedAxis 0 (CallFunction|AxisComponent (.HitComponent (Collision|BreakHitResult _outhit)))))
        (:NewEnumerator0
          _)
        (:NewEnumerator1
          _)
        (:NewEnumerator2
          _))
      (Variables|Default|SetDragedLocation (Math|Transform|InverseTransformLocation (Math|Conversions|ToTransform(Vector) (Transformation|GetWorldLocation (.axiscomponent (Utilities|Struct|MakeDragedAxis 0 (CallFunction|AxisComponent (.HitComponent (Collision|BreakHitResult _outhit))))))) (.Location (Collision|BreakHitResult _outhit))))))
  (:Released
    (if _movefunction
      (Variables|Default|SetAxis%20Draged 0))))

(event Input|KeyboardEvents|M
  (params (Key :type Key%20Structure :default "None"))
  (:Pressed
    (bind _output_get (Variables|Default|SetMoveFunction (not (Variables|Default|GetMoveFunction))))
    (Variables|/Script/Engine.PlayerController|SetbShowMouseCursor (Game|GetPlayerController 0) _output_get)))

(fn ConstructionScript)

(fn AxisComponent
  (params (Axis%20Component :type Primitive%20Component%20Object%20Reference))
  (Variables|Default|SetAxis%20Draged Axis%20Component)
  (if (== (Variables|Default|GetAxis%20Draged) (Variables|Default|GetX))
    (return "NewEnumerator0")
    (elif (== (Variables|Default|GetAxis%20Draged) (Variables|Default|GetY))
      (return "NewEnumerator1")
      (elif (== (Variables|Default|GetAxis%20Draged) (Variables|Default|GetZ))
        (return "NewEnumerator2")))))