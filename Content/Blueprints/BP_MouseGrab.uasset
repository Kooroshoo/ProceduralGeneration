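; Controllable pawn with a G-toggled grab mode that shows the cursor and lets the mouse drag Movable components.
; Left click traces under the cursor, storing the component, hit distance, local grab offset and skeletal bone.
; Tick holds it at that distance along the cursor ray, using a PhysicsHandle with debug line for simulating bodies, SetWorldLocation otherwise.
; Axis inputs move the pawn along controller up/right vectors; look rotation is disconnected.
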(event EventBeginPlay
  (Development|PrintString "Press G to go into Grab Mode"))

(event EventTick
  (params (DeltaSeconds :type Float%20%28single-precision%29))
  (bind _returnvalue (Game|GetPlayerController 0))
  (bind _grabedcomponent (Variables|Default|GetGrabedComponent))
  (bind _originaldistancetoobject (Variables|Default|GetOriginalDistanceToObject))
  (bind (_worldlocation _worlddirection) (Game|Player|ConvertMouseLocationToWorldSpace _returnvalue))
  (bind _returnvalue_2 (Math|Float|Truncate _originaldistancetoobject))
  (bind _returnvalue_3 (* _worlddirection _returnvalue_2))
  (bind _returnvalue_4 (+ _worldlocation _returnvalue_3))
  (if (Variables|Default|GetGrabMode)
    (Utilities|IsValid (Variables|Default|GetGrabedComponent)
      (:Is%20Valid
        (if (Physics|IsSimulatingPhysics (Variables|Default|GetGrabedComponent) "None")
          (Physics|Components|PhysicsHandle|SetTargetLocation (Variables|Default|GetPhysicsHandle) _returnvalue_4)
          (Rendering|Debug|DrawDebugLine _returnvalue_4 (Math|Transform|TransformLocation (select (Variables|Default|GetSkeletalMesh) (Transformation|GetSocketTransform _grabedcomponent (Variables|Default|GetBoneName) "RTS_World") (Transformation|GetWorldTransform _grabedcomponent)) (Variables|Default|GetRelativeGrabLocation)) "(R=0.000000,G=1.000000,B=0.058191,A=1.000000)" 0.0 5.0)
          (else
            (Transformation|SetWorldLocation (Variables|Default|GetGrabedComponent) (Math|Transform|InverseTransformLocation (Math|Conversions|ToTransform(Vector) (Variables|Default|GetRelativeGrabLocation)) _returnvalue_4) false false)))))))

(event Input|AxisEvents|InputAxisTurn
  (params (AxisValue :type Float%20%28single-precision%29)))

(event Input|AxisEvents|InputAxisLookUp
  (params (AxisValue :type Float%20%28single-precision%29)))

(event Input|AxisEvents|InputAxisMoveRight
  (params (AxisValue :type Float%20%28single-precision%29))
  ;[1 1 1] Movement
  (Transformation|AddActorWorldOffset (* (Math|Vector|GetRightVector (Transformation|GetActorRotation (Pawn|GetController))) (* AxisValue 1e+01))))

(event Input|AxisEvents|InputAxisMoveForward
  (params (AxisValue :type Float%20%28single-precision%29))
  ;[1 1 1] Movement
  (Transformation|AddActorWorldOffset (* (Math|Vector|GetUpVector (Transformation|GetActorRotation (Pawn|GetController))) (* AxisValue 1e+01))))

(event Input|KeyboardEvents|G
  (params (Key :type Key%20Structure :default "None"))
  (bind _returnvalue (Game|GetPlayerController 0))
  (:Pressed
    (Variables|Default|SetGrabMode (not (Variables|Default|GetGrabMode)))
    (Variables|/Script/Engine.PlayerController|SetbShowMouseCursor _returnvalue (not (Variables|/Script/Engine.PlayerController|GetbShowMouseCursor _returnvalue)))))

(event Input|MouseEvents|LeftMouseButton
  (params (Key :type Key%20Structure :default "None"))
  (bind _returnvalue (Game|GetPlayerController 0))
  (bind _grabmode (Variables|Default|GetGrabMode))
  (bind (_worldlocation _worlddirection) (Game|Player|ConvertMouseLocationToWorldSpace _returnvalue))
  (:Pressed
    (if _grabmode
      (bind (_outhit _returnvalue_2) (Collision|LineTraceByChannel _worldlocation (+ _worldlocation (* _worlddirection 10000)) "TraceTypeQuery1" true 0 "ForDuration"))
      (if _returnvalue_2
        (if (== (Variables|/Script/Engine.SceneComponent|GetMobility (.HitComponent (Collision|BreakHitResult _outhit))) (Utilities|Enum|LiteralenumEComponentMobility "Movable"))
          (Variables|Default|SetOriginalDistanceToObject (.Distance (Collision|BreakHitResult _outhit)))
          (bind _output_get (Variables|Default|SetGrabedComponent (.HitComponent (Collision|BreakHitResult _outhit))))
          (if (Physics|IsSimulatingPhysics _output_get "None")
            (Utilities|Casting|CastToSkeletalMeshComponent (Variables|Default|GetGrabedComponent)
              (:then
                (Variables|Default|SetSkeletalMesh true)
                (Variables|Default|SetBoneName (.HitBoneName (Collision|BreakHitResult _outhit))))
              (:CastFailed
                _))
            (Class|PhysicsHandleComponent|GrabComponentatLocation (Variables|Default|GetPhysicsHandle) (Variables|Default|GetGrabedComponent) (Variables|Default|GetBoneName) (.Location (Collision|BreakHitResult _outhit)))
            (Variables|Default|SetRelativeGrabLocation (Math|Transform|InverseTransformLocation (select (Variables|Default|GetSkeletalMesh) (Transformation|GetSocketTransform (Variables|Default|GetGrabedComponent) (Variables|Default|GetBoneName) "RTS_World") (Transformation|GetWorldTransform (Variables|Default|GetGrabedComponent))) (.Location (Collision|BreakHitResult _outhit))))
            (else
              (Variables|Default|SetRelativeGrabLocation (Math|Transform|InverseTransformLocation (Math|Conversions|ToTransform(Vector) (Transformation|GetWorldLocation (.HitComponent (Collision|BreakHitResult _outhit)))) (.Location (Collision|BreakHitResult _outhit))))))))))
  (:Released
    (if _grabmode
      (Variables|Default|SetGrabedComponent 0)
      (Physics|Components|PhysicsHandle|ReleaseComponent (Variables|Default|GetPhysicsHandle)))))

(fn ConstructionScript)